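; BP_InteractionTest is a test actor that changes to a random color whenever it is interacted with.
; The construction script creates a dynamic instance of MAT_InteractionTest on its static mesh and applies the initial Color.
; Both regular and drone interaction events share one path that picks random RGB values, stores them in Color and updates the material parameter.
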(event EventOnDroneInteraction
  (bind _output_get (Variables|Default|SetColor (Utilities|Struct|MakeLinearColor (Math|Random|RandomFloatinRange 0.0 1.0) (Math|Random|RandomFloatinRange 0.0 1.0) (Math|Random|RandomFloatinRange 0.0 1.0) 1.0)))
  (Rendering|Material|SetVectorParameterValue (Variables|Default|GetMaterialInstance) "Color" _output_get :!class /Script/Engine.MaterialInstanceDynamic))

(event EventOnInteraction
  (params (Player :type Third%20Person%20Character%20Object%20Reference))
  (bind _output_get (Variables|Default|SetColor (Utilities|Struct|MakeLinearColor (Math|Random|RandomFloatinRange 0.0 1.0) (Math|Random|RandomFloatinRange 0.0 1.0) (Math|Random|RandomFloatinRange 0.0 1.0) 1.0)))
  (Rendering|Material|SetVectorParameterValue (Variables|Default|GetMaterialInstance) "Color" _output_get :!class /Script/Engine.MaterialInstanceDynamic))

(fn ConstructionScript
  (bind _returnvalue (Rendering|Material|CreateDynamicMaterialInstance (Variables|Default|GetStaticMesh) 0 "/Game/Systems/Interactions/MAT_InteractionTest.MAT_InteractionTest" "None" :!class /Script/Engine.PrimitiveComponent))
  (bind _output_get (Variables|Default|SetMaterialInstance _returnvalue))
  (Rendering|Material|SetVectorParameterValue _output_get "Color" (Variables|Default|GetColor) :!class /Script/Engine.MaterialInstanceDynamic))