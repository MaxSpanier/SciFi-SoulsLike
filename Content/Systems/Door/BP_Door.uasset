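; BP_Door is an interactable swinging door that opens away from or toward the player's side and closes on the next interaction.
; OnInteraction compares the door's forward vector with the direction to the player, using a loose equality tolerance to choose the swing sign.
; The Door_Open timeline scales SMDoor's relative yaw by Angle, playing or reversing according to Open.
; Open toggles on every timeline update.
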(event EventOnInteraction
  (params (Player :type Third%20Person%20Character%20Object%20Reference))
  (if (not (Variables|Default|GetOpen))
    (Variables|Default|SetDirection (Math|Vector|Equal(Vector) (Transformation|GetActorForwardVector) (Math|Vector|Normalize (- (Transformation|GetActorLocation (.AsThird%20Person%20Character (Utilities|Casting|CastToThirdPersonCharacter (Game|GetPlayerCharacter 0)))) (Transformation|GetActorLocation))) 1.0))
    (bind _newtrack_0 (Timeline|Door_Open Play)
      (:Update
        (Transformation|SetRelativeRotation (Variables|Default|GetSM_Door) (Math|Rotator|MakeRotator 0.0 0.0 (* _newtrack_0 (Variables|Default|GetAngle) (Math|Float|SelectFloat -1.0 1.0 (Variables|Default|GetDirection)))) false false)
        (Variables|Default|SetOpen (not (Variables|Default|GetOpen)))))
    (else
      (Timeline|Door_Open Reverse))))

(fn ConstructionScript)