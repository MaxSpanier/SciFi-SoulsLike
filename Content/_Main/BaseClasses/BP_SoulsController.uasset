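; BP_SoulsController is a controller Blueprint that creates the player's HUD and relays health and stamina changes to it.
; Shortly after BeginPlay, it creates W_PlayerUI for player controller 0, adds it to the viewport and initializes both bars to full.
; UpdateHealthUI and UpdateStaminaUI events pass new values to the stored widget's bar update functions.
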(event EventBeginPlay
  (Utilities|FlowControl|Delay 0.2)
  (Utilities|IsValid (Game|GetPlayerController 0)
    (:Is%20Valid
      (bind _returnvalue (UserInterface|CreateWidget "/Game/_Main/UI/W_PlayerUI.W_PlayerUI_C" (Game|GetPlayerController 0)))
      (bind _output_get (Variables|Default|SetPlayerUI _returnvalue))
      (UserInterface|Viewport|AddtoViewport _output_get 0)
      (CallFunction|UpdateHealthUI 1.0)
      (CallFunction|UpdateStaminaUI 1.0))))

(event EventUpdateStaminaUI
  (params (NewStamina :type Float%20%28single-precision%29))
  (Default|UpdateStaminaBar (Variables|Default|GetPlayerUI) NewStamina))

(event EventUpdateHealthUI
  (params (NewHealth :type Float%20%28single-precision%29))
  (Default|UpdateHealthBar (Variables|Default|GetPlayerUI) NewHealth))

(fn ConstructionScript)