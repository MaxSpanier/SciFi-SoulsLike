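; Security camera control panel that a player uses to view and cycle through a list of security cameras.
; On interaction it moves input from the player to itself and sets the view target to the first camera.
; Next and previous inputs cycle cameras with wraparound, while Interact returns view and input to the player.
; A looping timer polls a sphere for overlapping ThirdPersonCharacters to show or hide the interact prompt.
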(event EventBeginPlay
  (Utilities|Time|SetTimerbyFunctionName 0 "SetTextVisibility" 0.5 true))

(event EventOnInteraction
  (params (Player :type Third%20Person%20Character%20Object%20Reference))
  (bind _returnvalue (Pawn|GetController Player))
  (bind _asplayer_controller (Utilities|Casting|CastToPlayerController _returnvalue))
  (if (and (Private|HasCameras?) (not (Private|Occupied?)))
    (Variables|Default|SetOccupiedPlayer Player)
    (Input|DisableInput Player _asplayer_controller)
    (Input|EnableInput _asplayer_controller)
    (Variables|Default|SetActiveCameraIndex 0)
    (Private|SetViewTargetasActiveCamera)))

(event Input|ActionEvents|InputActionInteract
  (params (Key :type Key%20Structure))
  (:Pressed
    (Game|Player|SetViewTargetwithBlend (.AsPlayer%20Controller (Utilities|Casting|CastToPlayerController (Pawn|GetController (Variables|Default|GetOccupiedPlayer)))) (Variables|Default|GetOccupiedPlayer) 0.0 "VTBlend_Linear" 0.0 false)
    (Input|EnableInput (Variables|Default|GetOccupiedPlayer) (.AsPlayer%20Controller (Utilities|Casting|CastToPlayerController (Pawn|GetController (Variables|Default|GetOccupiedPlayer)))))
    (Input|DisableInput (.AsPlayer%20Controller (Utilities|Casting|CastToPlayerController (Pawn|GetController (Variables|Default|GetOccupiedPlayer)))))
    (Variables|Default|SetOccupiedPlayer 0)))

(event Input|ActionEvents|InputActionNextCamera
  (params (Key :type Key%20Structure))
  (:Pressed
    (Private|IncrementCameraIndex)
    (Private|SetViewTargetasActiveCamera)))

(event Input|ActionEvents|InputActionPreviousCamera
  (params (Key :type Key%20Structure))
  (:Pressed
    (Private|DecrementCameraIndex)
    (Private|SetViewTargetasActiveCamera)))

(fn ConstructionScript)

(fn HasCameras?
  (return (> (Utilities|Array|Length (Variables|Default|GetSecurityCameras)) 0)))

(fn Occupied?
  (return (Utilities|IsValid (Variables|Default|GetOccupiedPlayer))))

(fn SetViewTargetasActiveCamera
  (Game|Player|SetViewTargetwithBlend (.AsPlayer%20Controller (Utilities|Casting|CastToPlayerController (Pawn|GetController (Variables|Default|GetOccupiedPlayer)))) (Utilities|Array|Get(acopy) (Variables|Default|GetSecurityCameras) (Variables|Default|GetActiveCameraIndex)) 0.0 "VTBlend_Linear" 0.0 false))

(fn IncrementCameraIndex
  (if (> (+ (Variables|Default|GetActiveCameraIndex) 1) (Utilities|Array|LastIndex (Variables|Default|GetSecurityCameras)))
    (Variables|Default|SetActiveCameraIndex 0)
    (else
      (Math|Integer|IncrementInt (Variables|Default|GetActiveCameraIndex)))))

(fn DecrementCameraIndex
  (if (< (- (Variables|Default|GetActiveCameraIndex) 1) 0)
    (Variables|Default|SetActiveCameraIndex (Utilities|Array|LastIndex (Variables|Default|GetSecurityCameras)))
    (else
      (Math|Integer|DecrementInt (Variables|Default|GetActiveCameraIndex)))))

(fn SetTextVisibility
  (bind _interactmessage (Variables|Default|GetInteractMessage))
  (bind _array_element (Utilities|Array|ForEachLoopwithBreak (Collision|GetOverlappingActors (Variables|Default|GetSphere) 0 :!class /Script/Engine.PrimitiveComponent) :!label _label)
    (:LoopBody
      (Utilities|Casting|CastToThirdPersonCharacter _array_element)
      (Variables|Default|SetPlayerInTextRange true)
      (goto _label Break))
    (:Completed
      (if (Variables|Default|GetPlayerInTextRange)
        (Rendering|SetVisibility _interactmessage true false)
        (Variables|Default|SetPlayerInTextRange false)
        (else
          (Rendering|SetVisibility _interactmessage false false))))))