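; Health pickup actor that heals the player on overlap and loops a level sequence for its movement.
; Sphere overlap casts to BP_PlayerCharacter and, if health is below max, adds HealingAmount to the PlayerStats struct.
; Only when the heal reaches max does it clamp health, message the player controller to update health UI, print a debug string and destroy itself.
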(event OnComponentBeginOverlap(Sphere)
  (params (OverlappedComponent :type Primitive%20Component%20Object%20Reference) (OtherActor :type Actor%20Object%20Reference) (OtherComp :type Primitive%20Component%20Object%20Reference) (OtherBodyIndex :type Integer) (bFromSweep :type Boolean) (SweepResult :type Hit%20Result%20Structure%20%28by%20ref%29))
  (bind _asbp_player_character (Utilities|Casting|CastToBP_PlayerCharacter OtherActor))
  (if (< (.CurrentHealth (Utilities|Struct|BreakS_PlayerStats (Variables|/Game/_Main/Player/BP_PlayerCharacter.BP_PlayerCharacter_C|GetPlayerStats _asbp_player_character))) (.MaxHealth (Utilities|Struct|BreakS_PlayerStats (Variables|/Game/_Main/Player/BP_PlayerCharacter.BP_PlayerCharacter_C|GetPlayerStats _asbp_player_character))))
    (bind _structout (Utilities|Struct|SetmembersinS_PlayerStats (Variables|/Game/_Main/Player/BP_PlayerCharacter.BP_PlayerCharacter_C|GetPlayerStats _asbp_player_character) (+ (.CurrentHealth (Utilities|Struct|BreakS_PlayerStats (Variables|/Game/_Main/Player/BP_PlayerCharacter.BP_PlayerCharacter_C|GetPlayerStats _asbp_player_character))) (Variables|Default|GetHealingAmount))))
    (if (>= (.CurrentHealth (Utilities|Struct|BreakS_PlayerStats _structout)) (.MaxHealth (Utilities|Struct|BreakS_PlayerStats _structout)))
      (Utilities|Struct|SetmembersinS_PlayerStats _structout (.MaxHealth (Utilities|Struct|BreakS_PlayerStats _structout)))
      (Class|INTSoulsController|UpdateHealthUI(Message) (Game|GetPlayerController 0) (/ (.CurrentHealth (Utilities|Struct|BreakS_PlayerStats _structout)) (.MaxHealth (Utilities|Struct|BreakS_PlayerStats _structout))))
      (Development|PrintString "Healed Player")
      (Actor|DestroyActor))))

(event EventBeginPlay
  (bind _returnvalue (Sequencer|Player|CreateLevelSequencePlayer (Variables|Default|GetMovementSequence)))
  (Class|MovieSceneSequencePlayer|PlayLooping _returnvalue -1))

(fn ConstructionScript)